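; Lobby player controller that drives the local player's lobby UI.
; SetupLobbyMenu creates the LobbyMenu widget with the server name, shows the cursor and sets Game and UI input focused on the menu.
; ShowLoadingScreen removes that menu and adds a LoadingScreen widget in its place.
; InitialSetup, UpdateLobbySettings and CallUpdate are empty stubs, and LobbyPCRef simply returns the controller itself.
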(event Custom|InitialSetup)

(event Custom|SetupLobbyMenu
  (params (ServerName :type Text))
  (Variables|Default|SetbShowMouseCursor true)
  (bind _returnvalue (UserInterface|CreateWidget "/Game/_Main/Lobby/LobbyMenu.LobbyMenu_C" 0 ServerName))
  (bind _output_get (Variables|Default|SetLobbyWidget _returnvalue))
  (UserInterface|Viewport|AddtoViewport _output_get 0)
  (Input|SetInputModeGameandUI self (Variables|Default|GetLobbyWidget) "DoNotLock" true))

(event Custom|UpdateLobbySettings
  (params (MapImage :type Texture%202D%20Object%20Reference) (MapName :type Text) (MapTime :type Text)))

(event Custom|CallUpdate
  (params (PlayerSettings :type S%20Player%20Info%20Structure) (ChangedStatus? :type Boolean)))

(event Custom|ShowLoadingScreen
  (Widget|RemovefromParent (Variables|Default|GetLobbyWidget))
  (bind _returnvalue (UserInterface|CreateWidget "/Game/_Main/Widgets/LoadingScreen.LoadingScreen_C" self))
  (UserInterface|Viewport|AddtoViewport _returnvalue 0))

(fn ConstructionScript)

(fn LobbyPCRef
  (return self))