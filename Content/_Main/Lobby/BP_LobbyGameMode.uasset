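; BP_LobbyGameMode is the game mode for the Steam multiplayer lobby, setting up each player who joins.
; On PostLogin it records the controller, gathers PlayerStarts, reads server name and player limit from the game instance, then initializes that player's lobby menu and map display.
; It talks to game instance and controllers through reference-returning calls, and can show every player a loading screen.
; SpawnPlayer is called but still empty.
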(event Custom|SpawnPlayer
  (params (Player :type Player%20Controller%20Object%20Reference)))

(event Custom|StartLoadingScreen
  (for _array_element (Variables|Default|GetConnectedPlayers)
    (bind _lobbypc (Class|BPILobbyPC|LobbyPCRef(Message) _array_element))
    (Default|ShowLoadingScreen _lobbypc)))

(event EventPostLogin
  (params (NewPlayer :type Player%20Controller%20Object%20Reference))
  (bind _output_get (Variables|Default|SetConnectedPlayer NewPlayer))
  (Utilities|Array|AddUnique (Variables|Default|GetConnectedPlayers) _output_get)
  (bind _outactors (Actor|GetAllActorsOfClass "/Script/Engine.PlayerStart"))
  (Variables|Default|SetSpawnPoints _outactors)
  (bind _gameinstance (Class|BPIGameInstance|SteamGameInstanceRef(Message) (Game|GetGameInstance)))
  (Variables|Default|SetServerName (Variables|/Game/_Main/SteamGameInstance.SteamGameInstance_C|GetServerName _gameinstance))
  (Variables|Default|SetMaxPlayers (Variables|/Game/_Main/SteamGameInstance.SteamGameInstance_C|GetMaxPlayers _gameinstance))
  (bind _lobbypc (Class|BPILobbyPC|LobbyPCRef(Message) (Variables|Default|GetConnectedPlayer)))
  (Default|InitialSetup _lobbypc)
  (Default|SetupLobbyMenu _lobbypc (Variables|Default|GetServerName))
  (Default|UpdateLobbySettings _lobbypc (Variables|Default|GetDefaultMapImage) (Variables|Default|GetDefaultMapName) (Variables|Default|GetDefaultMapTime))
  (CallFunction|SpawnPlayer (Variables|Default|GetConnectedPlayer)))

(fn ConstructionScript)

(fn LobbyGMref
  (return self))